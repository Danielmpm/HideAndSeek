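; Hider ability component for a prop-hunt style mode, managing the owner's disguise mesh and three cooldown-gated abilities.
; The disguise starts random, can copy a camera-traced prop from RandomObjects or a Decoy's mesh, and can be force-rerolled by grenade impact.
; Triggers share an AbilityID-indexed check with timer resets, then spawn a smoke screen, an overlap-checked decoy, or turn nearby ReplaceableMeshActors into the current disguise.
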(event Custom|TriggerAbility1
  ;[1 1 1] Trigger Abilities
  (Variables|Default|SetAbilityID 0)
  (CallFunction|CheckforCooldown))

(event Custom|ChangeMesh
  ;[1 1 1] Change the mesh
  (for _array_element (Actor|GetComponentsByClass (Components|GetOwner) "/Script/Engine.CameraComponent")
    (bind _outhit (Collision|LineTraceForObjects (Transformation|GetActorLocation (Components|GetOwner)) (+ (Transformation|GetWorldLocation _array_element) (* (Math|Vector|GetForwardVector (.Rotation (Math|Transform|BreakTransform (Transformation|GetWorldTransform _array_element)))) 1000)) (Utilities|Array|MakeArray "ObjectTypeQuery1" "ObjectTypeQuery2") false 0 "Persistent"))
    (bind _astrap_decoy (Utilities|Casting|CastToTrap_Decoy (.HitActor (Collision|BreakHitResult _outhit)))
      (:then
        (bind _outactors (Actor|GetAllActorsOfClass "/Game/Blueprints/Sudeep/Trap_Decoy.Trap_Decoy_C"))
        (for _array_element_2 _outactors
          (if (== _array_element_2 _astrap_decoy)
            (Development|PrintString "Hello")))
        (CallFunction|SwitchMesh))
      (:CastFailed
        (CallFunction|SwitchMesh)))))

(event Custom|TriggerAbility2
  ;[1 1 1] Trigger Abilities
  (Variables|Default|SetAbilityID 1)
  (CallFunction|CheckforCooldown))

(event Custom|TriggerUltimate
  ;[1 1 1] Trigger Abilities
  (Variables|Default|SetAbilityID 2)
  (CallFunction|CheckforCooldown))

(event Custom|AssignInitialMesh
  (bind _random_objects (Variables|Default|GetRandom_Objects))
  ;[1 1 1] Call Initial Mesh
  (CallFunction|MeshSwap (Utilities|Array|Get(acopy) _random_objects (Math|Random|RandomIntegerinRange 0 (- (Utilities|Array|Length _random_objects) 1)))))

(event Custom|Reset2
  ;[1 1 1] Cooldown Over
  (Utilities|Array|SetArrayElem (Variables|Default|GetAbility_Available) 2 true))

(event Custom|CheckForCooldown
  (bind _returnvalue (Components|GetOwner))
  ;[1 1 1] Check Cooldown
  (if (Math|Boolean|Equal(Boolean) (Utilities|Array|Get(acopy) (Variables|Default|GetAbility_Available) (Variables|Default|GetAbilityID)) true)
    (if (== (Variables|Default|GetAbilityID) 1)
      (bind _returnvalue_2 (Class|KismetSystemLibrary|BoxOverlapActorsNEW (+ (+ (Transformation|GetActorLocation _returnvalue) "0.000000,0.000000,-70.000000") (* (Math|Vector|GetForwardVector (Transformation|GetActorRotation _returnvalue)) 150)) "40.000000,40.000000,20.000000" (Utilities|Array|MakeArray "ObjectTypeQuery1" "ObjectTypeQuery2")))
      (if (not _returnvalue_2)
        (CallFunction|ApplyCooldown :!label _label)
        (CallFunction|FireAbility))
      (else
        (goto _label)))))

(event Custom|ApplyCooldown
  (bind _abilityid (Variables|Default|GetAbilityID))
  ;[1 1 1] Apply Cooldown
  (Utilities|Array|SetArrayElem (Variables|Default|GetAbility_Available) _abilityid false)
  (switch int _abilityid
    (:0
      (Utilities|Time|SetTimerbyEvent (EventDispatchers|CreateEvent :!event Custom|Reset0) 3.0))
    (:1
      (Utilities|Time|SetTimerbyEvent (EventDispatchers|CreateEvent :!event Custom|Reset1) 3.0))
    (:2
      (Utilities|Time|SetTimerbyEvent (EventDispatchers|CreateEvent :!event Custom|Reset2) 5.0))))

(event Custom|Reset0
  ;[1 1 1] Cooldown Over
  (Utilities|Array|SetArrayElem (Variables|Default|GetAbility_Available) 0 true))

(event Custom|Reset1
  ;[1 1 1] Cooldown Over
  (Utilities|Array|SetArrayElem (Variables|Default|GetAbility_Available) 1 true))

(event Custom|MeshSwap
  (params (Mesh :type Static%20Mesh%20Object%20Reference))
  ;[1 1 1] Swap Mesh
  (bind _output_get (Variables|Default|SetCurrent_Object Mesh))
  (Components|StaticMesh|SetStaticMesh (Variables|Default|GetOwnersMesh) _output_get))

(event Custom|UltimateSwap
  (params (Mesh :type Static%20Mesh%20Component%20Object%20Reference))
  ;[1 1 1] Ultimate Swap
  (Components|StaticMesh|SetStaticMesh Mesh (Variables|Default|GetCurrent_Object)))

(fn ForceSwitch
  (bind _random_objects (Variables|Default|GetRandom_Objects))
  ;[1 1 1] Force Switch on Grenade Impact
  (while (== (stale _output_get) (Variables|/Script/Engine.StaticMeshComponent|GetStaticMesh (Variables|Default|GetOwnersMesh)))
    (bind _output_get (Variables|Default|SetCurrent_Object (Utilities|Array|Get(acopy) _random_objects (Math|Random|RandomIntegerinRange 0 (- (Utilities|Array|Length _random_objects) 1))))))
  (CallFunction|MeshSwap (Variables|Default|GetCurrent_Object)))

(fn FireAbility
  (bind _returnvalue (Components|GetOwner))
  (bind _returnvalue_2 (Components|GetOwner))
  (bind _returnvalue_3 (Transformation|GetActorLocation _returnvalue_2))
  (bind (_x _y) (Math|Vector|BreakVector _returnvalue_3))
  ;[1 1 1] Firing of Abilities and Cooldown
  (switch int (Variables|Default|GetAbilityID)
    (:0
      (Game|SpawnActorfromClass "/Game/Blueprints/Sudeep/Smoke_Screen.Smoke_Screen_C" (Math|Transform|MakeTransform (- (Transformation|GetActorLocation _returnvalue) "0,-50.000000, 0") (Transformation|GetActorRotation _returnvalue)) "AlwaysSpawn" 0 0))
    (:1
      (for _array_element (Actor|GetComponentsByClass _returnvalue_2 "/Script/Engine.CameraComponent")
        (Game|SpawnActorfromClass "/Game/Blueprints/Sudeep/Decoy.Decoy_C" (Math|Transform|MakeTransform (+ (+ _returnvalue_3 "0.000000,0.000000,-100.000000") (* (Math|Vector|Normalize (- (Math|Vector|MakeVector _x _y 0.0) (Math|Vector|MakeVector (.X (Math|Vector|BreakVector (Transformation|GetWorldLocation _array_element))) (.Y (Math|Vector|BreakVector (Transformation|GetWorldLocation _array_element))) 0.0))) 150)) "0, 0, 0" "1.000000,1,1.000000") "AlwaysSpawn" 0 0 0)))
    (:2
      (bind _outactors (Class|KismetSystemLibrary|SphereOverlapActorsNEW (Transformation|GetActorLocation (Components|GetOwner)) 5e+02 (Utilities|Array|MakeArray "ObjectTypeQuery2" "ObjectTypeQuery1")))
      (for _array_element_2 _outactors
        (bind _asreplaceable_mesh_actor (Utilities|Casting|CastToReplaceableMeshActor _array_element_2))
        (for _array_element_3 (Actor|GetComponentsByClass _asreplaceable_mesh_actor "/Script/Engine.StaticMeshComponent")
          (CallFunction|UltimateSwap _array_element_3))))))

(fn SwitchMesh
  ;[1 1 1] Switching Mesh
  (for _array_element (Actor|GetComponentsByClass (Components|GetOwner) "/Script/Engine.CameraComponent")
    (bind _outhit (Collision|LineTraceForObjects (Transformation|GetActorLocation (Components|GetOwner)) (+ (Transformation|GetWorldLocation _array_element) (* (Math|Vector|GetForwardVector (.Rotation (Math|Transform|BreakTransform (Transformation|GetWorldTransform _array_element)))) 1000)) (Utilities|Array|MakeArray "ObjectTypeQuery1" "ObjectTypeQuery2") false 0 "Persistent"))
    (bind _asstatic_mesh_actor (Utilities|Casting|CastToStaticMeshActor (.HitActor (Collision|BreakHitResult _outhit)))
      (:then
        (LocalVariables|SetstaticMesh (Variables|/Script/Engine.StaticMeshComponent|GetStaticMesh (Variables|/Script/Engine.StaticMeshActor|GetStaticMeshComponent _asstatic_mesh_actor)))
        (for (_array_element_2 _array_index) (Variables|Default|GetRandom_Objects) :!label _label
          (if (== _array_element_2 (LocalVariables|GetstaticMesh))
            (CallFunction|MeshSwap (Utilities|Array|Get(acopy) (Variables|Default|GetRandom_Objects) _array_index))
            (Audio|SpawnSoundatLocation "/Game/Sounds/Pop__Morph_.Pop__Morph_" (Transformation|GetActorLocation (Components|GetOwner))))))
      (:CastFailed
        (bind _asreplaceable_mesh_actor (Utilities|Casting|CastToReplaceableMeshActor (.HitActor (Collision|BreakHitResult _outhit)))
          (:then
            (LocalVariables|SetstaticMesh (Variables|/Script/Engine.StaticMeshComponent|GetStaticMesh (Variables|/Game/Blueprints/Daniel/RandomObjectsRoom/ReplaceableMeshActor.ReplaceableMeshActor_C|GetStaticMesh _asreplaceable_mesh_actor)))
            (goto _label))
          (:CastFailed
            (bind _outactors (Actor|GetAllActorsOfClass "/Game/Blueprints/Sudeep/Decoy.Decoy_C"))
            (for _array_element_3 _outactors
              (if (== _array_element_3 (.HitActor (Collision|BreakHitResult _outhit)))
                (for _array_element_4 (Actor|GetComponentsByClass _array_element_3 "/Script/Engine.StaticMeshComponent")
                  (CallFunction|MeshSwap (Variables|/Script/Engine.StaticMeshComponent|GetStaticMesh _array_element_4))
                  (Audio|SpawnSoundatLocation "/Game/Sounds/Pop__Morph_.Pop__Morph_" (Transformation|GetActorLocation (Components|GetOwner))))))))))))

(fn OnRepCurrentObject)