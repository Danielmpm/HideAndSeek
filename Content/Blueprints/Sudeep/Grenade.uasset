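; Grenade actor that, on impact, forces nearby Hiders to switch and then destroys itself.
; On a mesh hit, the server runs a sphere overlap at the hit point and calls ForceSwitch on each Hider's HiderAbilities component.
; It then plays a reveal sound at the impact location and calls Explode, which destroys the actor.
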(event `self.StaticMeshComponent.OnComponentHit`
  (params (OtherActor :type "Actor Object Reference") (OtherComp :type "PrimitiveComponent Object Reference") (NormalImpulse :type "Vector Structure") (Hit :type "HitResult Structure (by ref)"))
  (bind (_bblockinghit _binitialoverlap _time _location) (`GameplayStatics.BreakHitResult` Hit))
  ;[1 1 1] Hider Detection
  (`/Engine/EditorBlueprintResources/ActorMacros.Switch Has Authority`
    (:`Authority`
      (bind _outactors (`KismetSystemLibrary.SphereOverlapActors_NEW` _location 150.0 (`|MakeArray` "ObjectTypeQuery2" "ObjectTypeQuery3" :!type "EObjectTypeQuery Enum")))
      (for _array_element _outactors
        (bind _ashider (cast `/Game/HiderBP/Blueprints/Hider` _array_element))
        (`/Game/Blueprints/Sudeep/HiderAbilities.Force_Switch` (`/Game/HiderBP/Blueprints/Hider.HiderAbilities` _ashider)))
      (`GameplayStatics.PlaySoundAtLocation` "/Game/Sounds/16_bit_Grenade__Reveal_.16_bit_Grenade__Reveal_" _location)
      (`self.Explode`))))

(event `self.ReceiveActorBeginOverlap`
  (params (OtherActor :type "Actor Object Reference")))

(event `self.ReceiveTick`
  (params (DeltaSeconds :type "Float (single-precision)")))

(event `Explode`
  ;[1 1 1] Explode
  (`self.K2_DestroyActor`))

(fn `UserConstructionScript`)