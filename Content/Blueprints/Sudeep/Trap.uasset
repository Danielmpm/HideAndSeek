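; Trap actor that catches the first Hider to overlap its static mesh, flagging that Hider as trapped through its HiderAbilities.
; The catch plays closing and alarm sounds at the trap and starts a three-second, one-shot timer.
; DestroyTrap, the apparent timer callback, clears the Hider's trapped flag and destroys the actor, making the trap single-use.
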(event `self.StaticMeshComponent.OnComponentBeginOverlap`
  (params (OtherActor :type "Actor Object Reference") (OtherComp :type "PrimitiveComponent Object Reference") (OtherBodyIndex :type Integer) (bFromSweep :type Boolean) (SweepResult :type "HitResult Structure (by ref)"))
  (bind _returnvalue (`self.K2_GetActorLocation` self))
  ;[1 1 1] Trap Hider
  (bind _ashider (cast `/Game/HiderBP/Blueprints/Hider` OtherActor))
  (if (not (`self.IsTrapped`))
    (set `self.IsTrapped` true)
    (bind _output_get (set `self.HiderTrapped` _ashider))
    (set `/Game/Blueprints/Sudeep/HiderAbilities.Is_Trapped` true (`/Game/HiderBP/Blueprints/Hider.HiderAbilities` _output_get))
    (`GameplayStatics.SpawnSoundAtLocation` "/Game/Sounds/trap_closing.trap_closing" _returnvalue)
    (`KismetSystemLibrary.K2_SetTimerDelegate` (`|CreateDelegate` :!event `DestroyTrap`) 3.0)
    (`GameplayStatics.PlaySoundAtLocation` "/Game/Sounds/3_second_Fire_Alarm.3_second_Fire_Alarm" _returnvalue)))

(event `self.ReceiveBeginPlay`)

(event `self.ReceiveActorBeginOverlap`
  (params (OtherActor :type "Actor Object Reference")))

(event `self.ReceiveTick`
  (params (DeltaSeconds :type "Float (single-precision)")))

(event `DestroyTrap`
  ;[1 1 1] Delete Trap
  (set `/Game/Blueprints/Sudeep/HiderAbilities.Is_Trapped` false (`/Game/HiderBP/Blueprints/Hider.HiderAbilities` (`self.HiderTrapped`)))
  (`self.K2_DestroyActor`))

(fn `UserConstructionScript`)