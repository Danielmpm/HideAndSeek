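; Seeker ability component that gives its owner two abilities: launching a Grenade or a Trap_Grenade.
; Each trigger event sets an AbilityID, then fires only if that slot in the AbilityAvailable array is true.
; Firing marks the slot unavailable, starts a per-ability one-shot cooldown timer, and spawns the projectile at LaunchPoint using the owner's rotation.
; Separate reset events re-enable each slot.
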(event `TriggerAbility1`
  ;[1 1 1] Comment
  (set `self.AbilityID` 0)
  (`self.CheckForCooldown` :!label _label))

(event `CheckForCooldown`
  ;[1 1 1] Check Cooldown
  (if (== (`KismetArrayLibrary.Array_Get` (`self.Ability_Available`) (`self.AbilityID`)) true)
    (`self.ApplyCooldown`)
    (`self.Fire_Ability`)))

(event `TriggerAbility2`
  ;[1 1 1] Comment
  (set `self.AbilityID` 1)
  (goto _label))

(event `Reset0`
  ;[1 1 1] Cooldown Over
  (`KismetArrayLibrary.Array_Set` (`self.Ability_Available`) 0 true))

(event `ApplyCooldown`
  (bind _abilityid (`self.AbilityID`))
  ;[1 1 1] Apply Cooldown
  (`KismetArrayLibrary.Array_Set` (`self.Ability_Available`) _abilityid false)
  (switch `int` _abilityid
    (:`0`
      (`KismetSystemLibrary.K2_SetTimerDelegate` (`|CreateDelegate` :!event `Reset0`) 3.0))
    (:`1`
      (`KismetSystemLibrary.K2_SetTimerDelegate` (`|CreateDelegate` :!event `Reset1`) 3.0))))

(event `Reset1`
  ;[1 1 1] Cooldown Over
  (`KismetArrayLibrary.Array_Set` (`self.Ability_Available`) 1 true))

(fn `Fire_Ability`
  (bind _returnvalue (`KismetMathLibrary.MakeTransform` (`Actor.K2_GetActorLocation` (`self.Launch_Point`)) (`Actor.K2_GetActorRotation` (`self.GetOwner`)) (0.5 0.5 0.5)))
  ;[1 1 1] Firing of Abilities and Cooldown
  (switch `int` (`self.AbilityID`)
    (:`0`
      (`|SpawnActorFromClass` "/Game/Blueprints/Sudeep/Grenade.Grenade_C" _returnvalue "Undefined" "OverrideRootScale"))
    (:`1`
      (`|SpawnActorFromClass` "/Game/Blueprints/Sudeep/Trap_Grenade.Trap_Grenade_C" _returnvalue "Undefined" "OverrideRootScale"))))