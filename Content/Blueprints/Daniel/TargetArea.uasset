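; TargetArea is a replicated area actor that a manager can time while players stand inside, though its overlap logic is marked not working.
; The IsActive RepNotify shows or hides the graphics, clearing any started timer either way.
; Authority-only overlap events check IsActive but do nothing.
; Disconnected logic would count players, start a timer calling the Manager's AreaFinished on first entry, and cancel it once empty.
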(event `self.ReceiveActorBeginOverlap`
  (params (OtherActor :type "Actor Object Reference"))
  ;[1 1 1] not working
  (`/Engine/EditorBlueprintResources/ActorMacros.Switch Has Authority`
    (:`Authority`
      (if (`self.IsActive`)
        _))))

(event `self.ReceiveActorEndOverlap`
  (params (OtherActor :type "Actor Object Reference"))
  ;[1 1 1] not working
  (`/Engine/EditorBlueprintResources/ActorMacros.Switch Has Authority`
    (:`Authority`
      (if (`self.IsActive`)
        _))))

(event `self.ReceiveTick`
  (params (DeltaSeconds :type "Float (single-precision)"))
  ;[1 1 1] not working
)

(fn `ActivateArea`
  (`SceneComponent.SetVisibility` (`self.Graphics`) true false)
  (if (`self.timerStarted`)
    (`KismetSystemLibrary.K2_ClearTimerHandle` (`self.TimerHandle`))))

(fn `DeactivateArea`
  (`SceneComponent.SetVisibility` (`self.Graphics`) false false)
  (if (`self.timerStarted`)
    (`KismetSystemLibrary.K2_ClearTimerHandle` (`self.TimerHandle`))))

(fn `OnRep_IsActive`
  (if (`self.IsActive`)
    (`self.ActivateArea`)
    (else
      (`self.DeactivateArea`))))

(fn `UserConstructionScript`)