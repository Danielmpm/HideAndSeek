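; Lobby player controller for a hide-and-seek game, linking the lobby menu widget to session handling in HideNSeek_GameInstance.
; Shortly after BeginPlay, it creates the menu and shows the mouse cursor, only with authority.
; Host, join and session-refresh functions forward to the game instance, and NotifySessionListUpdated refreshes the widget's list.
; Hosting is authority-only, while JoinGame ignores its SessionIndex input and always joins index 0.
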(event `self.ReceiveBeginPlay`
  (`KismetSystemLibrary.Delay` 0.2)
  (`self.CreateUI`))

(event `CreateUI`
  (`/Engine/EditorBlueprintResources/ActorMacros.Switch Has Authority`
    (:`Authority`
      (bind _returnvalue (`|CreateWidget` "/Game/UI/Lobby_Menu.Lobby_Menu_C" self))
      (bind _output_get (set `self.LobbyMenuWidget` _returnvalue))
      (`UserWidget.AddToViewport` _output_get 0)
      (`Widget.SetVisibility` _returnvalue "Visible")
      (set `self.bShowMouseCursor` true))))

(fn `HostGame`
  (params (LevelName :type Name))
  (`/Engine/EditorBlueprintResources/ActorMacros.Switch Has Authority`
    (:`Authority`
      (bind _ashide_nseek_game_instance (cast `/Game/Blueprints/Daniel/HideNSeek_GameInstance` (`GameplayStatics.GetGameInstance`)))
      (`/Game/Blueprints/Daniel/HideNSeek_GameInstance.Instance_HostLobby` _ashide_nseek_game_instance self LevelName)
      (`WidgetBlueprintLibrary.SetInputMode_GameAndUIEx` self))))

(fn `JoinGame`
  (params (SessionIndex :type Integer))
  (bind _ashide_nseek_game_instance (cast `/Game/Blueprints/Daniel/HideNSeek_GameInstance` (`GameplayStatics.GetGameInstance`)))
  (`/Game/Blueprints/Daniel/HideNSeek_GameInstance.Instance_JoinLobby` _ashide_nseek_game_instance self 0))

(fn `NotifySessionListUpdated`
  (`/Game/UI/Lobby_Menu.UpdateAvailableSessionsList` (`self.LobbyMenuWidget`)))

(fn `UpdateSessionList`
  (bind _ashide_nseek_game_instance (cast `/Game/Blueprints/Daniel/HideNSeek_GameInstance` (`GameplayStatics.GetGameInstance`)))
  (`/Game/Blueprints/Daniel/HideNSeek_GameInstance.Instance_UpdateAvailableSessions` _ashide_nseek_game_instance self))

(fn `UserConstructionScript`)