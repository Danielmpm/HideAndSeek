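; HideNSeek game instance that handles multiplayer sessions for hosting, finding and joining lobbies.
; Hosting creates a five-connection session, LAN optional, then opens the given level as a listen server.
; Searching is LAN-only and capped at one result, caching AvailableSessions on success and notifying the requesting player on success or failure.
; Joining uses a supplied search result, and all outcomes except successful hosting print debug messages.
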(event `Instance_HostLobby`
  (params (Caller :type "PlayerController Object Reference") (Level :type Name) (useLan :type Boolean))
  (`CreateSessionCallbackProxy.CreateSession` Caller 5 useLan
    (:`OnSuccess`
      (`GameplayStatics.OpenLevel` Level true "listen"))
    (:`OnFailure`
      (`KismetSystemLibrary.PrintString` "Failed creating session" true true (struct :`R` 1.0 :`G` 0.043975 :`A` 1.0)))))

(event `Instance_JoinLobby`
  (params (Player :type "PlayerController Object Reference") (Session :type "BlueprintSessionResult Structure"))
  (`JoinSessionCallbackProxy.JoinSession` Player Session
    (:`OnSuccess`
      (`KismetSystemLibrary.PrintString` "Joining"))
    (:`OnFailure`
      (`KismetSystemLibrary.PrintString` "Failed to Join Session"))))

(event `Instance_UpdateAvailableSessions`
  (params (Player :type "/Game/Blueprints/Daniel/Lobby/LobbyPlayerController Object Reference"))
  (bind _results (`FindSessionsCallbackProxy.FindSessions` Player 1 true)
    (:`OnSuccess`
      (set `self.AvailableSessions` _results))
    (:`OnFailure`
      (`KismetSystemLibrary.PrintString` "Session search failed" true true (struct :`R` 1.0 :`G` 0.028582 :`A` 1.0))))
  (`/Game/Blueprints/Daniel/Lobby/LobbyPlayerController.NotifySessionListUpdated` Player)
  (`KismetSystemLibrary.PrintString` "SessionListUpdated"))