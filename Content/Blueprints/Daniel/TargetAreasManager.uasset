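; Manager actor that runs a match's sequence of TargetArea objectives, keeping one randomly chosen area active at a time.
; On BeginPlay it gathers every TargetArea, deactivates it and registers itself as manager, then starts the match after a short delay, activating areas only on authority.
; Picks are removed from a pool that refills when empty; AreaFinished advances to the next until the TotalAreas countdown runs out.
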(event `self.ReceiveBeginPlay`
  (bind _outactors (`GameplayStatics.GetAllActorsOfClass` "/Game/Blueprints/Daniel/TargetArea.TargetArea_C"))
  (bind _output_get (set `self.TargetAreas` _outactors))
  (for _array_element _output_get
    (set `/Game/Blueprints/Daniel/TargetArea.IsActive` false _array_element)
    (set `/Game/Blueprints/Daniel/TargetArea.Manager` self _array_element)
    (set `self.remainingAreasNumber` (`self.TotalAreas`))
    (`KismetSystemLibrary.Delay` 2.0)
    (`self.TargetAreas_StartMatch`))
  (set `self.RemainingAreas` _output_get))

(event `TargetAreas_StartMatch`
  (`/Engine/EditorBlueprintResources/ActorMacros.Switch Has Authority`
    (:`Authority`
      (`self.ActivateNewArea`))))

(event `self.ReceiveActorBeginOverlap`
  (params (OtherActor :type "Actor Object Reference")))

(event `self.ReceiveTick`
  (params (DeltaSeconds :type "Float (single-precision)")))

(fn `ActivateNewArea`
  (bind _remainingareas (`self.RemainingAreas`))
  (bind _returnvalue (`KismetArrayLibrary.Array_Length` _remainingareas))
  (if (> (`KismetArrayLibrary.Array_Length` (`self.TargetAreas`)) 0)
    (if (> _returnvalue 0) :!label _label
      (if (!= (`self.ActiveArea`) null)
        (`/Game/Blueprints/Daniel/TargetArea.DeactivateArea` (`self.ActiveArea`)))
      (bind _output_get (set `self.ActiveArea` (`KismetArrayLibrary.Array_Get` _remainingareas (`KismetMathLibrary.RandomIntegerInRange` 0 (- _returnvalue 1)))))
      (set `/Game/Blueprints/Daniel/TargetArea.IsActive` true _output_get)
      (`KismetArrayLibrary.Array_RemoveItem` (`self.RemainingAreas`) _output_get)
      (else
        (set `self.RemainingAreas` (`self.TargetAreas`))
        (goto _label)))
    (else
      (`KismetSystemLibrary.PrintString` "No Areas Found!!" true true (struct :`R` 1.0 :`G` 0.195585 :`A` 1.0)))))

(fn `AreaFinished`
  (set `/Game/Blueprints/Daniel/TargetArea.IsActive` false (`self.ActiveArea`))
  (bind _output_get (set `self.remainingAreasNumber` (- (`self.remainingAreasNumber`) 1)))
  (if (> _output_get 0)
    (`self.ActivateNewArea`)
    (else
      (`KismetSystemLibrary.PrintString` "No More Areas Left"))))

(fn `UserConstructionScript`)